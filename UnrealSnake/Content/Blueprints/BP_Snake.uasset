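; Player-steered snake actor that moves continuously along its forward vector once any of the four move inputs is pressed.
; Tick applies a swept, teleporting location offset of MoveSpeed per frame, without delta-time scaling.
; Each input passes a world-axis direction to SetDirection, which rotates the actor unless CanMoveInThisDirection finds it reverses the current heading.
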(event EventTick
  (params (DeltaSeconds :type Float%20%28single-precision%29))
  (if (Variables|Default|GetStartedMoving)
    (Transformation|SetActorLocation (+ (Transformation|GetActorLocation) (* (Transformation|GetActorForwardVector) (Math|Conversions|ToVector(Float) (Variables|Default|GetMoveSpeed)))) true true)))

(event Input|ActionEvents|InputActionMoveUp
  (params (Key :type Key%20Structure :default "None"))
  (:Pressed
    (CallFunction|SetDirection (Math|Vector|GetForwardVector "0, 0, 0"))))

(event Input|ActionEvents|InputActionMoveDown
  (params (Key :type Key%20Structure :default "None"))
  (:Pressed
    (CallFunction|SetDirection (Math|Vector|NegateVector (Math|Vector|GetForwardVector "0, 0, 0")))))

(event Input|ActionEvents|InputActionMoveLeft
  (params (Key :type Key%20Structure :default "None"))
  (:Pressed
    (CallFunction|SetDirection (Math|Vector|NegateVector (Math|Vector|GetRightVector "0, 0, 0")))))

(event Input|ActionEvents|InputActionMoveRight
  (params (Key :type Key%20Structure :default "None"))
  (:Pressed
    (CallFunction|SetDirection (Math|Vector|GetRightVector "0, 0, 0"))))

(event Input|ActionEvents|InputActionMoveUp
  (params (Key :type Key%20Structure :default "None"))
  (:Pressed
    (Variables|Default|SetStartedMoving true)))

(event Input|ActionEvents|InputActionMoveDown
  (params (Key :type Key%20Structure :default "None"))
  (:Pressed
    (Variables|Default|SetStartedMoving true)))

(event Input|ActionEvents|InputActionMoveLeft
  (params (Key :type Key%20Structure :default "None"))
  (:Pressed
    (Variables|Default|SetStartedMoving true)))

(event Input|ActionEvents|InputActionMoveRight
  (params (Key :type Key%20Structure :default "None"))
  (:Pressed
    (Variables|Default|SetStartedMoving true)))

(fn ConstructionScript)

(fn CanMoveinThisDirection
  (params (NewDirection :type Vector))
  (return (Utilities|Operators|NotEqual(!=) NewDirection (Math|Vector|NegateVector (Transformation|GetActorForwardVector)) 0.5)))

(fn SetDirection
  (params (New%20Direction :type Vector))
  (bind _result (CallFunction|CanMoveinThisDirection New%20Direction))
  (if _result
    (Transformation|SetActorRotation (Math|Conversions|RotationFromXVector New%20Direction))))