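; Game mode for a grid-based Snake game that handles setup, scoring, snake speed and game over.
; On BeginPlay it finds the grid and item spawner, loads the high score, then spawns the snake at its starting cell.
; Each consumed item triggers the next spawn and a score increment, with a flag skipping the initial spawn.
; When the snake stops, it saves any new high score and swaps the score widget for game-over UI.
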(event Custom|OnSnakeStopped
  (bind _returnvalue (Game|GetPlayerController 0))
  (CallFunction|SaveHighScore)
  (bind _foundwidgets (Widget|GetAllWidgetsOfClass "/Game/Blueprints/Widgets/WBP_Score.WBP_Score_C" true))
  (for _array_element _foundwidgets
    (Widget|RemovefromParent _array_element))
  (bind _returnvalue_2 (UserInterface|CreateWidget "/Game/Blueprints/Widgets/WBP_GameOver.WBP_GameOver_C"))
  (UserInterface|Viewport|AddtoViewport _returnvalue_2 0)
  (Variables|/Script/Engine.PlayerController|SetbShowMouseCursor _returnvalue true)
  (Input|SetInputModeUIOnly _returnvalue _returnvalue_2 "DoNotLock"))

(event Custom|OnConsumableItemDestroyed
  (bind _item (Default|SpawnConsumableItem (Variables|Default|GetGridItemSpawner)))
  (EventDispatchers|BindEventtoOnConsumed _item (delegate Custom|OnConsumableItemDestroyed))
  (if (Variables|Default|GetIsGameStarted)
    (Math|Integer|IncrementInt (Variables|Default|GetScore))
    (else
      (Variables|Default|SetIsGameStarted true))))

(event Custom|OnPlay
  (bind _snake (Variables|Default|GetSnake))
  (switch Utilities|FlowControl|Switch|SwitchonE_SnakeSpeed (Variables|Default|GetSnakeSpeed)
    (:NewEnumerator0
      (Variables|/Game/Blueprints/Snake/BP_Snake.BP_Snake_C|SetMoveSpeed _snake 1e+01))
    (:NewEnumerator1
      (Variables|/Game/Blueprints/Snake/BP_Snake.BP_Snake_C|SetMoveSpeed _snake 2e+01))))

(event EventBeginPlay
  (CallFunction|GetActors)
  (CallFunction|LoadHighScore)
  (Utilities|FlowControl|Delay 0.1)
  (CallFunction|InitializePlayer)
  (CallFunction|OnConsumableItemDestroyed))

(fn ConstructionScript)

(fn GetActors
  (bind _returnvalue (Actor|GetActorOfClass "/Game/Blueprints/BP_Grid.BP_Grid_C"))
  (Variables|Default|SetGrid _returnvalue)
  (bind _returnvalue_2 (Actor|GetActorOfClass "/Game/Blueprints/BP_GridItemSpawner.BP_GridItemSpawner_C"))
  (Variables|Default|SetGridItemSpawner _returnvalue_2))

(fn InitializePlayer
  (bind _cell (Default|GetCellbyGridLocation (Variables|Default|GetGrid) (Variables|Default|GetStartingRow) (Variables|Default|GetStartingColumn)))
  (bind _returnvalue (Game|SpawnActorfromClass "/Game/Blueprints/Snake/BP_Snake.BP_Snake_C" (Math|Transform|MakeTransform (Transformation|GetActorLocation _cell)) "Undefined" 0 0))
  (bind _output_get (Variables|Default|SetSnake _returnvalue))
  (EventDispatchers|BindEventtoOnStopped _output_get (EventDispatchers|CreateEvent :!event Custom|OnSnakeStopped)))

(fn LoadHighScore
  (bind _returnvalue (SaveGame|DoesSaveGameExist (Variables|Default|GetSaveSlotName)))
  (if _returnvalue
    (bind _returnvalue_2 (SaveGame|LoadGamefromSlot (Variables|Default|GetSaveSlotName)))
    (bind _asbp_high_score (Utilities|Casting|CastToBP_HighScore _returnvalue_2))
    (Variables|Default|SetHighScore (Variables|/Game/Blueprints/BP_HighScore.BP_HighScore_C|GetScore _asbp_high_score))))

(fn SaveHighScore
  (if (> (Variables|Default|GetScore) (Variables|Default|GetHighScore))
    (bind _returnvalue (SaveGame|CreateSaveGameObject "/Game/Blueprints/BP_HighScore.BP_HighScore_C"))
    (bind _output_get (Variables|/Game/Blueprints/BP_HighScore.BP_HighScore_C|SetScore _returnvalue (Variables|Default|GetScore)))
    (Variables|Default|SetHighScore _output_get)
    (SaveGame|SaveGametoSlot _returnvalue (Variables|Default|GetSaveSlotName))))