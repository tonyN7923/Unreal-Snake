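; BP_Grid is a grid actor that spawns a Rows by Columns board of BP_GridCell actors on BeginPlay, attached to its root.
; Cells live in a flat array, so neighbor lookups step by one for Up/Down and by Rows for Left/Right, falling back to the current cell on invalid indices.
; It also serves random cells, optionally skipping occupied ones, and row/column lookups, which use Columns as stride and thus assume a square grid.
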(event EventBeginPlay
  (CallFunction|InitializeGrid))

(fn ConstructionScript)

(fn InitializeGrid
  (bind _cellsize (Variables|Default|GetCellSize))
  (for _index (range 0 (- (Variables|Default|GetColumns) 1))
    (for _index_2 (range 0 (- (Variables|Default|GetRows) 1))
      (bind _returnvalue (Game|SpawnActorfromClass "/Game/Blueprints/BP_GridCell.BP_GridCell_C" (Math|Transform|MakeTransform (Math|Vector|MakeVector (Math|Conversions|ToFloat(Integer) (* _cellsize _index_2)) (Math|Conversions|ToFloat(Integer) (* _index _cellsize)) 0.0)) "Undefined" 0 0))
      (Utilities|Array|Add (Variables|Default|GetCells) _returnvalue)
      (Transformation|AttachComponentToComponent _returnvalue (Variables|Default|GetDefaultSceneRoot) "None" "KeepWorld" "KeepWorld" "KeepWorld" false))))

(fn GetRandomCell
  (params (IncludeOccupied :type Boolean))
  (bind _output_get (LocalVariables|SetTempCells (Variables|Default|GetCells)))
  (Utilities|Array|Shuffle _output_get)
  (bind _array_element (Utilities|Array|ForEachLoopwithBreak (LocalVariables|GetTempCells) :!label _label)
    (:LoopBody
      (if IncludeOccupied
        (return _array_element)
        (elif (not (Variables|/Game/Blueprints/BP_GridCell.BP_GridCell_C|GetIsOccupied _array_element))
          (goto _label Break))))
    (:Completed
      (return _array_element))))

(fn GetNextCellPosition
  (params (CurrentCell :type BP%20Grid%20Cell%20Object%20Reference) (Direction :type E_Direction%20Enum :default "NewEnumerator0"))
  (bind _rows (Variables|Default|GetRows))
  (bind _index (CallFunction|GetCellIndex CurrentCell))
  (switch Utilities|FlowControl|Switch|SwitchonE_Direction Direction
    (:NewEnumerator0
      (if (not (== (Math|Integer|%(Integer) _index _rows) (- _rows 1)))
        (bind _position (CallFunction|GetCellPositionfromCurrentCell CurrentCell 1))
        (return _position)))
    (:NewEnumerator1
      (if (not (== (Math|Integer|%(Integer) _index _rows) 0))
        (bind _position_2 (CallFunction|GetCellPositionfromCurrentCell CurrentCell -1))
        (return _position_2)))
    (:NewEnumerator2
      (bind _position_3 (CallFunction|GetCellPositionfromCurrentCell CurrentCell (- 0 (Variables|Default|GetRows))))
      (return _position_3))
    (:NewEnumerator3
      (bind _position_4 (CallFunction|GetCellPositionfromCurrentCell CurrentCell (Variables|Default|GetRows)))
      (return _position_4))))

(fn GetCellPositionfromCurrentCell
  (params (CurrentCell :type BP%20Grid%20Cell%20Object%20Reference) (StepFromCurrentIndex :type Integer))
  (bind _index (CallFunction|GetCellIndex CurrentCell))
  (bind _position (CallFunction|GetCellbyIndex (+ _index StepFromCurrentIndex) CurrentCell))
  (return _position))

(fn GetCellIndex
  (params (Cell :type BP%20Grid%20Cell%20Object%20Reference))
  (return (Utilities|Array|FindItem (Variables|Default|GetCells) Cell)))

(fn GetCellbyIndex
  (params (Index :type Integer) (DefaultCell :type BP%20Grid%20Cell%20Object%20Reference))
  (bind _output_get (LocalVariables|SetCellResult (Utilities|Array|Get(acopy) (Variables|Default|GetCells) Index)))
  (Utilities|IsValid _output_get
    (:Is%20Valid
      (return (LocalVariables|GetCellResult) (Transformation|GetActorLocation (LocalVariables|GetCellResult))))
    (:Is%20Not%20Valid
      (return DefaultCell (Transformation|GetActorLocation DefaultCell)))))

(fn GetCellbyGridLocation
  (params (Row :type Integer) (Column :type Integer))
  (bind _cell (CallFunction|GetCellbyIndex (+ (- Row 1) (* (Variables|Default|GetColumns) (- Column 1)))))
  (return _cell))