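; BP_GridItemSpawner is an actor that spawns consumable items and obstacles on the level's grid.
; On BeginPlay it finds and caches the BP_Grid actor.
; SpawnConsumableItem and SpawnObstacle each pick a random class from their own array, get a random cell from the grid, and spawn at that cell's location.
; Spawns ignore collisions, and both functions return the new actor to the caller.
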(event EventBeginPlay
  (bind _returnvalue (Actor|GetActorOfClass "/Game/Blueprints/BP_Grid.BP_Grid_C"))
  (Variables|Default|SetGrid _returnvalue))

(fn ConstructionScript)

(fn SpawnConsumableItem
  (bind _cell (Default|GetRandomCell (Variables|Default|GetGrid) false))
  (bind _returnvalue (Game|SpawnActorfromClass (.OutItem (Utilities|Array|Random (Variables|Default|GetConsumableItems))) (Math|Transform|MakeTransform (Transformation|GetActorLocation _cell)) "AlwaysSpawn" 0 0))
  (return _returnvalue))

(fn SpawnObstacle
  (bind _cell (Default|GetRandomCell (Variables|Default|GetGrid) false))
  (bind _returnvalue (Game|SpawnActorfromClass (.OutItem (Utilities|Array|Random (Variables|Default|GetObstacles))) (Math|Transform|MakeTransform (Transformation|GetActorLocation _cell)) "AlwaysSpawn" 0 0))
  (return _returnvalue))