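; BP_SnakeHead is the head part of the snake and decides what happens when the snake runs into something.
; Its CellDetector overlap event casts the other actor: a consumable item makes the Snake grow and plays a bite sound.
; Overlapping another snake part or an obstacle stops the Snake's movement, while any other actor is ignored.
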(event OnComponentBeginOverlap(CellDetector)
  (params (OverlappedComponent :type Primitive%20Component%20Object%20Reference) (OtherActor :type Actor%20Object%20Reference) (OtherComp :type Primitive%20Component%20Object%20Reference) (OtherBodyIndex :type Integer) (bFromSweep :type Boolean) (SweepResult :type Hit%20Result%20Structure%20%28by%20ref%29))
  (Utilities|Casting|CastToBP_ConsumableItem OtherActor
    (:then
      (Default|Grow (Variables|Default|GetSnake))
      (Audio|PlaySound2D "/Game/Audio/S_Bite.S_Bite" 1.0 1.0 0.0 0 0))
    (:CastFailed
      (Utilities|Casting|CastToBP_SnakePart OtherActor
        (:then
          (Default|StopMoving (Variables|Default|GetSnake)))
        (:CastFailed
          (Utilities|Casting|CastToBP_Obstacle OtherActor)
          (Default|StopMoving (Variables|Default|GetSnake)))))))

(fn ConstructionScript
  (|CallParentFunction))