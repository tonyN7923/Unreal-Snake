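; BP_SnakeSkinPalette is a snake skin palette that supplies a color for an element at a given index in an array.
; GetColor switches on the SkinPattern setting and reads from the Pattern color array.
; Round Robin cycles through the colors, Gradient interpolates from first to last color across the array length, and Dual gives index zero the first color and all others the second.
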(fn ConstructionScript)

(fn GetColor
  (params (Index :type Integer) (ArrayLength :type Integer))
  (bind _pattern (Variables|Default|GetPattern))
  (switch Utilities|FlowControl|Switch|SwitchonE_SkinPattern (Variables|Default|GetSkinPattern)
    (:NewEnumerator0
      (return (Utilities|Array|Get(acopy) (Variables|Default|GetPattern) (Math|Integer|%(Integer) Index (Utilities|Array|Length (Variables|Default|GetPattern))))))
    (:NewEnumerator1
      (LocalVariables|SetStartGradientColor (Utilities|Array|Get(acopy) (Variables|Default|GetPattern)))
      (LocalVariables|SetEndGradientColor (Utilities|Array|Get(acopy) _pattern (Utilities|Array|LastIndex _pattern)))
      (return (Math|Conversions|ToLinearColor(Vector) (Math|Vector|Lerp(Vector) (Math|Conversions|ToVector(LinearColor) (LocalVariables|GetStartGradientColor)) (Math|Conversions|ToVector(LinearColor) (LocalVariables|GetEndGradientColor)) (/ (Math|Conversions|ToFloat(Integer) Index) (Math|Conversions|ToFloat(Integer) (- ArrayLength 1)))))))
    (:NewEnumerator2
      (if (== Index 0)
        (return (Utilities|Array|Get(acopy) (Variables|Default|GetPattern)))
        (else
          (return (Utilities|Array|Get(acopy) (Variables|Default|GetPattern) 1)))))))